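; Base Blueprint for card actors, providing health and server-side target tracking.
; Any damage is subtracted from Health, with no death check.
; On authority, TargetRange overlaps set CurrentTarget when IsNotTargetingTower is false and CanTarget passes, a stub that always returns true.
; When the current target leaves range, that flag resets to false if set, but CurrentTarget is not cleared.
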(event `self.ReceiveAnyDamage`
  (params (Damage :type "Float (single-precision)") (DamageType :type "DamageType Object Reference") (InstigatedBy :type "Controller Object Reference") (DamageCauser :type "Actor Object Reference"))
  (set `self.Health` (- (`self.Health`) Damage)))

(event `self.TargetRange.OnComponentBeginOverlap`
  (params (OverlappedComponent :type "PrimitiveComponent Object Reference") (OtherActor :type "Actor Object Reference") (OtherComp :type "PrimitiveComponent Object Reference") (OtherBodyIndex :type Integer) (bFromSweep :type Boolean) (SweepResult :type "HitResult Structure (by ref)"))
  (`/Engine/EditorBlueprintResources/ActorMacros.Switch Has Authority`
    (:`Authority`
      (if (`self.IsNotTargetingTower`)
        _
        (elif (`self.CanTarget` OtherActor)
          (set `self.CurrentTarget` OtherActor))))))

(event `self.TargetRange.OnComponentEndOverlap`
  (params (OverlappedComponent :type "PrimitiveComponent Object Reference") (OtherActor :type "Actor Object Reference") (OtherComp :type "PrimitiveComponent Object Reference") (OtherBodyIndex :type Integer))
  (`/Engine/EditorBlueprintResources/ActorMacros.Switch Has Authority`
    (:`Authority`
      (if (and (`self.IsNotTargetingTower`) (== OtherActor (`self.CurrentTarget`)))
        (set `self.IsNotTargetingTower` false)))))

(fn `CanTarget`
  (params (NewTarget :type "Actor Object Reference"))
  (returns (CanTarget :type Boolean))
  (return true))

(fn `UserConstructionScript`)