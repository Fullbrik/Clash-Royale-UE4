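; Behavior tree service that copies combat state from a Card_Base actor into the blackboard.
; Each tick it casts the owner actor to Card_Base and writes its health, current target and tower-targeting flag to blackboard keys.
; The tower flag is stored as the inverse of IsNotTargetingTower, and nothing is written if the cast fails.
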(event `self.ReceiveTick`
  (params (OwnerActor :type "Actor Object Reference") (DeltaSeconds :type "Float (single-precision)"))
  (bind _ascard_base (cast `/Game/Blueprints/Cards/Card_Base` OwnerActor))
  (`BTFunctionLibrary.SetBlackboardValueAsFloat` (`self.HealthKey`) (`/Game/Blueprints/Cards/Card_Base.Health` _ascard_base))
  (`BTFunctionLibrary.SetBlackboardValueAsObject` (`self.TargetKey`) (`/Game/Blueprints/Cards/Card_Base.CurrentTarget` _ascard_base))
  (`BTFunctionLibrary.SetBlackboardValueAsBool` (`self.IsTargetingTowerKey`) (not (`/Game/Blueprints/Cards/Card_Base.IsNotTargetingTower` _ascard_base))))